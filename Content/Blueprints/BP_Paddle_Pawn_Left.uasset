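; BP_Paddle_Pawn_Left is the pawn for the left paddle, moved along the X axis by player input.
; Each Tick it applies a physics force to PaddleMesh, scaled by the Move_1 axis.
; If the actor passes either movement limit, it is placed just inside that bound and its linear velocity is zeroed instead of receiving force.
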(event `self.ReceiveTick`
  (params (DeltaSeconds :type "Float (single-precision)"))
  (bind _returnvalue (`self.K2_GetActorLocation`))
  (bind _movlimhigh (`self.MovLimHigh`))
  (bind _movlimitlow (`self.MovLimitLow`))
  (if (> (.x _returnvalue) _movlimhigh)
    (`self.K2_SetActorLocation` (`KismetMathLibrary.MakeVector` (- _movlimhigh 1.0) (.y _returnvalue) (.z _returnvalue)))
    (`PrimitiveComponent.SetPhysicsLinearVelocity` (`self.Paddle_Mesh`) (0.0 0.0 0.0) false "None")
    (elif (> _movlimitlow (.x _returnvalue))
      (`self.K2_SetActorLocation` (`KismetMathLibrary.MakeVector` (+ _movlimitlow 1.0) (.y _returnvalue) (.z _returnvalue)))
      (`PrimitiveComponent.SetPhysicsLinearVelocity` (`self.Paddle_Mesh`) (0.0 0.0 0.0) false "None")
      (else
        (`PrimitiveComponent.AddForce` (`self.Paddle_Mesh`) (`KismetMathLibrary.MakeVector` (* 100 (`self.GetInputAxisValue`))) "None" false)))))

(fn `UserConstructionScript`)