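; BP_Ball is the ball for a Pong-style paddle game, moved by setting its static mesh's physics velocity.
; BeginPlay launches it in a randomized direction scaled by BallVelocity, always toward negative Y.
; On overlap, either paddle flips Y and sets X from the hit offset relative to the paddle, giving angled returns.
; Horizontal borders flip X, while both goals only flip Y, with no scoring or reset here.
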(event `self.ReceiveBeginPlay`
  (bind _ballvelocity (`self.BallVelocity`))
  (bind _returnvalue (`KismetMathLibrary.RandomFloatInRange` (* 0.3 _ballvelocity) _ballvelocity))
  (`PrimitiveComponent.SetPhysicsLinearVelocity` (`self.StaticMesh`) (`KismetMathLibrary.MakeVector` (- _ballvelocity _returnvalue) (* -1 _returnvalue)) false "None"))

(event `self.ReceiveActorBeginOverlap`
  (params (OtherActor :type "Actor Object Reference"))
  (bind _ballvelocity (`self.BallVelocity`))
  (bind _asbp_paddle_pawn_left (cast `/Game/Blueprints/BP_Paddle_Pawn_Left` OtherActor)
    (:`then`
      (bind _returnvalue (`PrimitiveComponent.GetPhysicsLinearVelocity` (`self.StaticMesh`) "None"))
      (bind _result (`/Engine/EditorBlueprintResources/StandardMacros.NegateFloat` (.y _returnvalue))
        (:`  `
          (`PrimitiveComponent.SetPhysicsLinearVelocity` (`self.StaticMesh`) (`KismetMathLibrary.MakeVector` (* (- (.x (`self.K2_GetActorLocation`)) (.x (`self.K2_GetActorLocation` _asbp_paddle_pawn_left))) (/ _ballvelocity 180.0)) _result (.z _returnvalue)) false "None"))))
    (:`CastFailed`
      (bind _asbp_paddle_right (cast `/Game/Blueprints/BP_PaddleRight` OtherActor)
        (:`then`
          (bind _returnvalue_2 (`PrimitiveComponent.GetPhysicsLinearVelocity` (`self.StaticMesh`) "None"))
          (bind _result_2 (`/Engine/EditorBlueprintResources/StandardMacros.NegateFloat` (.y _returnvalue_2))
            (:`  `
              (`PrimitiveComponent.SetPhysicsLinearVelocity` (`self.StaticMesh`) (`KismetMathLibrary.MakeVector` (* (- (.x (`self.K2_GetActorLocation`)) (.x (`self.K2_GetActorLocation` _asbp_paddle_right))) (/ _ballvelocity 180.0)) _result_2 (.z _returnvalue_2)) false "None"))))
        (:`CastFailed`
          (cast `/Game/Blueprints/BP_HorBorder` OtherActor
            (:`then`
              (bind _returnvalue_3 (`PrimitiveComponent.GetPhysicsLinearVelocity` (`self.StaticMesh`) "None"))
              (bind _result_3 (`/Engine/EditorBlueprintResources/StandardMacros.NegateFloat` (.x _returnvalue_3))
                (:`  `
                  (`PrimitiveComponent.SetPhysicsLinearVelocity` (`self.StaticMesh`) (`KismetMathLibrary.MakeVector` _result_3 (.y _returnvalue_3) (.z _returnvalue_3)) false "None"))))
            (:`CastFailed`
              (cast `/Game/Blueprints/BP_LeftGoal` OtherActor
                (:`then`
                  _)
                (:`CastFailed`
                  (cast `/Game/Blueprints/BP_RightGoal` OtherActor)))
              (bind _returnvalue_4 (`PrimitiveComponent.GetPhysicsLinearVelocity` (`self.StaticMesh`) "None"))
              (bind _result_4 (`/Engine/EditorBlueprintResources/StandardMacros.NegateFloat` (.y _returnvalue_4))
                (:`  `
                  (`PrimitiveComponent.SetPhysicsLinearVelocity` (`self.StaticMesh`) (`KismetMathLibrary.MakeVector` (.x _returnvalue_4) _result_4 (.z _returnvalue_4)) false "None"))))))))))

(fn `UserConstructionScript`)